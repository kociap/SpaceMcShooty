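; Laser turret that aims a cannon in the YZ plane and fires Laser_projectile actors with a cooldown timer.
; RotateTowardsPoints rolls the barrel toward a point, clamped to a half circle.
; TryShoot, gated by MayShoot, spawns a projectile at the spawner, sets its velocity and rotation along the shot direction, and squashes the barrel.
; Tick advances the shot timer, which drives an eased barrel-scale recovery as recoil feedback.
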(event `self.ReceiveTick`
  (params (DeltaSeconds :type "Float (single-precision)"))
  (`self.update_timers` DeltaSeconds)
  (`self.restore_scale`))

(event `self.try_shoot`
  ;[1 1 1] shoot
  (if (`self.may_shoot`)
    (set `self.shot_timer` 0.0)
    (bind _returnvalue (`|SpawnActorFromClass` "/Game/blueprints/laser_projectile.laser_projectile_C" (`KismetMathLibrary.MakeTransform` (`SceneComponent.K2_GetComponentLocation` (`self.projectile_spawner`)) (struct) (0.2 0.2 0.2)) "Undefined" "OverrideRootScale" null null))
    (bind _laser_beam (`/Game/blueprints/laser_projectile.laser_beam` _returnvalue))
    (`PrimitiveComponent.SetAllPhysicsLinearVelocity` _laser_beam (* (`self.compute_shot_direction`) (`self.projectile_speed`)) false)
    (`SceneComponent.K2_SetWorldRotation` _laser_beam (`KismetMathLibrary.RotatorFromAxisAndAngle` (1.0 0.0 0.0) (`KismetMathLibrary.DegAtan2` (* (.y (`self.compute_shot_direction`)) -1.0) (.z (`self.compute_shot_direction`)))) false false)
    (`SceneComponent.SetRelativeScale3D` (`self.cannon_Cylinder_001`) (1.0 1.0 0.5))))

(event `self.rotate_towards_points`
  (params (point :type "Vector Structure"))
  ;[1 1 1] rotate
  (`SceneComponent.K2_SetWorldRotation` (`self.cannon_Cylinder_001`) (`KismetMathLibrary.RotatorFromAxisAndAngle` (1.0 0.0 0.0) (`KismetMathLibrary.DegAtan2` (* (.y (- point (`SceneComponent.K2_GetComponentLocation` (`self.DefaultSceneRoot`)))) -1.0) (.z (- point (`SceneComponent.K2_GetComponentLocation` (`self.DefaultSceneRoot`)))))) false false)
  (`SceneComponent.K2_SetRelativeRotation` (`self.cannon_Cylinder_001`) (`KismetMathLibrary.MakeRotator` (`KismetMathLibrary.ClampAngle` (.roll (`SceneComponent.RelativeRotation` (`self.cannon_Cylinder_001`))) -90.0 90.0)) false false))

(fn `restore_scale`
  (`SceneComponent.SetRelativeScale3D` (`self.cannon_Cylinder_001`) (`KismetMathLibrary.MakeVector` 1.0 1.0 (`|EaseFunction` "CircularOut" (`KismetMathLibrary.FClamp` (/ (`self.shot_timer`) (`self.shot_cooldown`))) 0.5 0.75))))

(fn `update_timers`
  (params (delta_time :type "Float (double-precision)"))
  (set `self.shot_timer` (+ delta_time (`self.shot_timer`))))

(fn `UserConstructionScript`
  (`parent.UserConstructionScript`))