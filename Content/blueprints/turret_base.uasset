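; Turret base that the player rotates and fires, serving as a mount for swappable turrets.
; On BeginPlay it spawns a Cannon and attaches it to the Body through AttachTurret, which detaches any current turret and returns it.
; Move axis input is smoothed by interpolation and rolls the Scene around the world X axis each tick, scaled by MoveSpeed without delta time.
; Shoot axis input past a threshold calls TryShoot on the attached turret.
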(event `self.ReceiveBeginPlay`
  ;[1 1 1] attach default turret
  (bind _returnvalue (`|SpawnActorFromClass` "/Game/blueprints/cannon.cannon_C" (`KismetMathLibrary.MakeTransform` (0.0 0.0 21.0)) "Undefined" "OverrideRootScale" null null))
  (`self.attach_turret` _returnvalue))

(event `InputAxis|move`
  (params (AxisValue :type "Float (single-precision)"))
  ;[1 1 1] smooth the fucking input
  (set `self.move_axis_smoothed` (+ (`self.move_axis_smoothed`) (* (- AxisValue (`self.move_axis_smoothed`)) (`self.smooth_factor`)))))

(event `self.ReceiveTick`
  (params (DeltaSeconds :type "Float (single-precision)"))
  ;[1 1 1] turn the fucking thing
  (`SceneComponent.K2_AddWorldRotation` (`self.Scene`) (`KismetMathLibrary.RotatorFromAxisAndAngle` (1.0 0.0 0.0) (* (`self.move_axis_smoothed`) (`self.move_speed`))) false false))

(event `InputAxis|shoot`
  (params (AxisValue :type "Float (single-precision)"))
  ;[1 1 1] shoot
  (if (>= AxisValue 0.5)
    (`/Game/blueprints/turret_type.try_shoot` (`self.attached_turret`))))

(fn `attach_turret`
  (params (turret :type "/Game/blueprints/turret_type Object Reference"))
  (returns (old_turret :type "/Game/blueprints/turret_type Object Reference"))
  (locals (previous_turret :type "/Game/blueprints/turret_type Object Reference"))
  (`/Engine/EditorBlueprintResources/StandardMacros.IsValid` (`self.attached_turret`)
    (:`Is Valid`
      (`SceneComponent.K2_DetachFromComponent` (`Actor.RootComponent` (`self.attached_turret`)) "KeepRelative" "KeepRelative" "KeepRelative" true)
      (set `local.previous_turret` (`self.attached_turret`)))
    (:`Is Not Valid`
      _))
  (`self.K2_AttachToComponent` turret (`self.body`) "None" "KeepRelative" "KeepRelative" "KeepRelative" true)
  (set `self.attached_turret` turret)
  (return (`local.previous_turret`)))

(fn `UserConstructionScript`)