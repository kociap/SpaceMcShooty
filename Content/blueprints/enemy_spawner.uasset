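; Enemy spawner actor that sends timed waves of enemies toward Earth at the world origin and registers itself with the custom player controller.
; Tick advances timers; when spawning is enabled and the cooldown passes, it spawns enemies at random points on a YZ-plane ring.
; Wave size, speed (capped) and spawn rate grow with elapsed time.
; Each enemy's collision box gets velocity toward Earth, matching roll and a flipped Z scale.
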(event `self.ReceiveBeginPlay`
  (bind _asplayer_controller_custom (cast `/Game/blueprints/player_controller_custom` (`GameplayStatics.GetPlayerController` 0)))
  (set `/Game/blueprints/player_controller_custom.enemy_spawner` self _asplayer_controller_custom))

(event `self.ReceiveTick`
  (params (DeltaSeconds :type "Float (single-precision)"))
  (`self.update_timers` DeltaSeconds)
  (if (`self.may_spawn`)
    (set `self.enemy_spawn_timer` 0.0)
    (for _ (range 1 (+ (`KismetMathLibrary.FFloor` (+ (`self.spawn_count`) (/ (`self.elapsed_time`) 60.0))) 1))
      (bind _enemy (`self.spawn_enemy_random_position` (`self.spawn_radius`)))
      (bind _collision_box (`/Game/blueprints/enemy.collision_box` _enemy))
      (bind _direction (`self.direction_towards_earth` _enemy))
      (`PrimitiveComponent.SetAllPhysicsLinearVelocity` _collision_box (* _direction (`KismetMathLibrary.FClamp` (+ (`self.enemy_speed`) (* (`self.elapsed_time`) 60.0)) 0.0 600.0)) false)
      (`SceneComponent.SetWorldScale3D` _collision_box (`self.compute_flip_factor` _direction))
      (`SceneComponent.K2_SetWorldRotation` _collision_box (`KismetMathLibrary.MakeRotator` (`KismetMathLibrary.DegAtan2` (.z _direction) (* (.y _direction) -1.0))) false false))))

(fn `spawn_enemy`)

(fn `spawn_enemy_random_position`
  (params (spawn_radius :type "Float (double-precision)"))
  (returns (enemy :type "/Game/blueprints/enemy Object Reference"))
  (bind _returnvalue (`|SpawnActorFromClass` "/Game/blueprints/enemy.enemy_C" (`KismetMathLibrary.MakeTransform` (* (`KismetMathLibrary.Normal` (`KismetMathLibrary.MakeVector` 0.0 (`KismetMathLibrary.RandomFloatInRange` -1.0 1.0) (`KismetMathLibrary.RandomFloatInRange` -1.0 1.0))) spawn_radius)) "Undefined" "OverrideRootScale" null null))
  (return _returnvalue))

(fn `update_timers`
  (params (delta_time :type "Float (double-precision)"))
  (set `self.enemy_spawn_timer` (+ delta_time (`self.enemy_spawn_timer`)))
  (set `self.elapsed_time` (+ delta_time (`self.elapsed_time`))))

(fn `UserConstructionScript`)