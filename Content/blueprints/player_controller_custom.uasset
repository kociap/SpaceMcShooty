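; Custom player controller that sets game-and-UI input, registers itself with Score and runs the game's defeat sequence.
; Defeat stops turret targeting and shooting, disables enemy spawning and fades out the music.
; While defeated, Tick drives every enemy's physics velocity along the line to Earth at the origin, using an ease-in-back curve for a brief pull-away before the plunge.
; Once no enemies remain, it allows restart.
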(event `self.ReceiveBeginPlay`
  (`WidgetBlueprintLibrary.SetInputMode_GameAndUIEx` self null "DoNotLock" false)
  (set `/Game/blueprints/score.player_controller` self (`self.score`)))

(event `self.ReceiveTick`
  (params (DeltaSeconds :type "Float (single-precision)"))
  (if (`self.is_defeated`)
    (bind _outactors (`GameplayStatics.GetAllActorsOfClass` "/Game/blueprints/enemy.enemy_C"))
    (if (> (`KismetArrayLibrary.Array_Length` _outactors) 0)
      (for _array_element _outactors
        (bind _collision_box (`/Game/blueprints/enemy.collision_box` _array_element))
        (`PrimitiveComponent.SetAllPhysicsLinearVelocity` _collision_box (* (`self.direction_towards_earth` (`SceneComponent.K2_GetComponentLocation` _collision_box)) (* 2000.0 (`self.ease_in_back` (`self.enemy_ease`)))) false))
      (set `self.enemy_ease` (`KismetMathLibrary.FClamp` (+ (`self.enemy_ease`) 0.005) -1.0))
      (else
        (set `self.allow_restart` true)))))

(fn `defeat`
  (if (not (`self.is_defeated`))
    (set `self.is_defeated` true)
    (for _array_element (`self.automatic_turrets`)
      (set `/Game/blueprints/automatic_turret.should_target` false _array_element))
    (`AudioComponent.FadeOut` (`self.music`) 2.0 0.0)
    (set `/Game/blueprints/enemy_spawner.spawning_enabled` false (`self.enemy_spawner`))
    (set `/Game/blueprints/turret_base.shooting_enabled` false (`self.turret_base`))))

(fn `direction_towards_earth`
  (params (pos :type "Vector Structure"))
  (returns (direction :type "Vector Structure"))
  (return (`KismetMathLibrary.Normal` (- (0.0 0.0 0.0) pos))))

(fn `ease_in_back`
  (params (t :type "Float (double-precision)"))
  (returns (ease :type "Float (double-precision)"))
  (return (* (* t t) (- (* t (+ 1.70158 1.0)) 1.70158))))

(fn `UserConstructionScript`)