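; HUD blueprint that puts the game's UI widget on screen and provides a pause toggle.
; On BeginPlay it creates the widget for player controller 0, adds it to the viewport and registers itself as that custom controller's Hud.
; TogglePause flips the paused state, then re-reads it, setting the GamePaused element visible when unpaused and hidden when paused.
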(event `self.ReceiveBeginPlay`
  (bind _returnvalue (`|CreateWidget` "/Game/blueprints/ui.ui_C" (`GameplayStatics.GetPlayerController` 0)))
  (bind _output_get (set `self.ui` _returnvalue))
  (`UserWidget.AddToViewport` _output_get 0)
  (bind _asplayer_controller_custom (cast `/Game/blueprints/player_controller_custom` (`GameplayStatics.GetPlayerController` 0)))
  (set `/Game/blueprints/player_controller_custom.hud` self _asplayer_controller_custom))

(fn `toggle_pause`
  (bind _returnvalue (not (`GameplayStatics.IsGamePaused`)))
  (bind _game_paused (`/Game/blueprints/ui.game_paused` (`self.ui`)))
  (`GameplayStatics.SetGamePaused` _returnvalue)
  (if _returnvalue
    (`Widget.SetVisibility` _game_paused "Visible")
    (else
      (`Widget.SetVisibility` _game_paused "Hidden"))))

(fn `UserConstructionScript`)