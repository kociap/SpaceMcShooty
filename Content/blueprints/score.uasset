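; Score-keeping Blueprint with a single AddPoints function that updates points and the on-screen counter.
; Non-negative inputs are added to TotalScore, while negative ones leave it unchanged.
; In either case, Points is then added to itself, and that value, not TotalScore, goes to the player controller's HUD text with a "Points:" prefix.
; BeginPlay and Tick are unused.
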(fn `add_points`
  (params (points :type Integer))
  (if (>= points 0)
    (set `self.total_score` (+ points (`self.total_score`))))
  (bind _output_get (set `self.points` (+ points (`self.points`))))
  (`TextBlock.SetText` (`/Game/blueprints/ui.points` (`/Game/blueprints/hud.ui` (`/Game/blueprints/player_controller_custom.hud` (`self.player_controller`)))) (`KismetTextLibrary.Conv_StringToText` (`KismetStringLibrary.BuildString_Int` "" "Points: " _output_get))))