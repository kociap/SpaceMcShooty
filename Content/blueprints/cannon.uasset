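; Cannon actor that fires physics-driven Cannon_ball projectiles, with a squash-and-recover recoil on the barrel.
; TryShoot, gated by MayShoot, resets the shot timer, spawns a ball at ProjectileSpawner, sets its velocity from ComputeShotDirection and ProjectileSpeed, and squashes the cylinder.
; Tick advances the timer and eases the cylinder's Z scale back over the cooldown.
; RotateTowardsPoints is empty; the cooldown and direction helpers contain only unconnected expressions.
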(event `self.ReceiveTick`
  (params (DeltaSeconds :type "Float (single-precision)"))
  (`self.update_timers` DeltaSeconds)
  (`self.restore_scale`))

(event `self.try_shoot`
  ;[1 1 1] shoot
  (if (`self.may_shoot`)
    (set `self.shot_timer` 0.0)
    (bind _returnvalue (`|SpawnActorFromClass` "/Game/blueprints/cannon_ball.cannon_ball_C" (`KismetMathLibrary.MakeTransform` (`SceneComponent.K2_GetComponentLocation` (`self.projectile_spawner`)) (struct) (0.2 0.2 0.2)) "Undefined" "OverrideRootScale" null null))
    (`PrimitiveComponent.SetAllPhysicsLinearVelocity` (`/Game/blueprints/cannon_ball.cannon_ball_mesh` _returnvalue) (* (`self.compute_shot_direction`) (`self.projectile_speed`)) false)
    (`SceneComponent.SetRelativeScale3D` (`self.cannon_Cylinder_001`) (1.0 1.0 0.5))))

(event `self.rotate_towards_points`
  (params (point :type "Vector Structure")))

(fn `restore_scale`
  (`SceneComponent.SetRelativeScale3D` (`self.cannon_Cylinder_001`) (`KismetMathLibrary.MakeVector` 1.0 1.0 (`|EaseFunction` "CircularOut" (`KismetMathLibrary.FClamp` (/ (`self.shot_timer`) (`self.shot_cooldown`))) 0.5 0.75))))

(fn `update_timers`
  (params (delta_time :type "Float (double-precision)"))
  (set `self.shot_timer` (+ delta_time (`self.shot_timer`))))

(fn `UserConstructionScript`
  (`parent.UserConstructionScript`))