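; Tree destruction Blueprint that animates a chosen tree shrinking away.
; Each Tick advances an ease value, normalised to 60 fps via delta time, until it reaches one.
; The cached scale is multiplied by one minus a hand-written ease-in-back curve, so the tree swells slightly before collapsing toward zero.
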(event `self.ReceiveTick`
  (params (DeltaSeconds :type "Float (single-precision)"))
  (if (< (`self.scale_ease`) 1.0)
    (`SceneComponent.SetWorldScale3D` (`self.chosen_tree`) (* (`self.cached_scale`) (- 1.0 (`self.ease_in_back` (`self.scale_ease`)))))
    (set `self.scale_ease` (+ (`self.scale_ease`) (* (/ DeltaSeconds 0.016666) 0.03)))))

(fn `ease_in_back`
  (params (A :type "Float (double-precision)"))
  (returns (ease :type "Float (double-precision)"))
  (return (* (* A A) (- (* A (+ 1.70158 1.0)) 1.70158))))

(fn `UserConstructionScript`)