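; Automatic turret mount that aims an attached, swappable turret at enemies and fires it.
; Each Tick while targeting is enabled, it keeps its target while valid and within rotation range, otherwise picking the closest Enemy in range on the outward side relative to world origin.
; A circular ease-in turns the turret, which tries to shoot once the ease completes.
; AttachTurret detaches any current turret, attaches the new one to Body and returns the previous.
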(event `self.ReceiveTick`
  (params (DeltaSeconds :type "Float (single-precision)"))
  (bind _attached_turret (`self.attached_turret`))
  (bind _attached_turret_2 (`self.attached_turret`))
  (bind (_negative _positive) (`/Game/blueprints/turret_type.get_rotation_range` _attached_turret_2))
  ;[1 1 1] turn the other fucking thing
  (if (`self.should_target`)
    (`/Engine/EditorBlueprintResources/StandardMacros.IsValid` (`self.targeted_enemy`)
      (:`Is Valid`
        (bind _angle (`/Game/blueprints/turret_type.compute_target_rotation` _attached_turret_2 (`SceneComponent.K2_GetComponentLocation` (`/Game/blueprints/enemy.collision_box` (`self.targeted_enemy`)))))
        (if (not (`self.in_range` _angle _negative _positive))
          (bind _enemy (`self.find_closest_enemy` :!label _label))
          (`/Engine/EditorBlueprintResources/StandardMacros.IsValid` _enemy
            (:`Is Valid`
              (set `self.targeted_enemy` _enemy)
              (set `self.turn_ease_factor` 0.0)))))
      (:`Is Not Valid`
        (goto _label)))
    (bind _angle_2 (`/Game/blueprints/turret_type.compute_target_rotation` _attached_turret (`SceneComponent.K2_GetComponentLocation` (`/Game/blueprints/enemy.collision_box` (`self.targeted_enemy`)))))
    (`/Game/blueprints/turret_type.set_relative_rotation` (`self.attached_turret`) (`|EaseFunction` "CircularIn" (`self.turn_ease_factor`) (`/Game/blueprints/turret_type.get_current_turn_angle` _attached_turret) _angle_2))
    (bind _output_get (set `self.turn_ease_factor` (`KismetMathLibrary.FClamp` (+ (`self.turn_ease_factor`) (* (`self.smoothing_speed`) (/ DeltaSeconds 0.016667))))))
    (if (`KismetMathLibrary.NearlyEqual_FloatFloat` _output_get 1.0)
      (`/Game/blueprints/turret_type.try_shoot` (`self.attached_turret`)))))

(fn `attach_turret`
  (params (turret :type "/Game/blueprints/turret_type Object Reference"))
  (returns (old_turret :type "/Game/blueprints/turret_type Object Reference"))
  (locals (previous_turret :type "/Game/blueprints/turret_type Object Reference"))
  (`/Engine/EditorBlueprintResources/StandardMacros.IsValid` (`self.attached_turret`)
    (:`Is Valid`
      (`SceneComponent.K2_DetachFromComponent` (`Actor.RootComponent` (`self.attached_turret`)) "KeepRelative" "KeepRelative" "KeepRelative" true)
      (set `local.previous_turret` (`self.attached_turret`)))
    (:`Is Not Valid`
      _))
  (`self.K2_AttachToComponent` turret (`self.body`) "None" "KeepRelative" "KeepRelative" "KeepRelative" true)
  (set `self.attached_turret` turret)
  (return (`local.previous_turret`)))

(fn `find_closest_enemy`
  (returns (enemy :type "/Game/blueprints/enemy Object Reference"))
  (locals (closest_enemy :type "/Game/blueprints/enemy Object Reference") (shortest_distance :type "Float (double-precision)" :default 100000000.0))
  (bind _attached_turret (`self.attached_turret`))
  (bind (_negative _positive) (`/Game/blueprints/turret_type.get_rotation_range` _attached_turret))
  (bind _returnvalue (`SceneComponent.K2_GetComponentLocation` (`/Game/blueprints/turret_type.DefaultSceneRoot` (`self.attached_turret`))))
  (bind _outactors (`GameplayStatics.GetAllActorsOfClass` "/Game/blueprints/enemy.enemy_C"))
  (for _array_element _outactors
    (bind _returnvalue_2 (`SceneComponent.K2_GetComponentLocation` (`/Game/blueprints/enemy.collision_box` _array_element)))
    (bind _angle (`/Game/blueprints/turret_type.compute_target_rotation` _attached_turret _returnvalue_2))
    (bind _returnvalue_3 (- _returnvalue_2 _returnvalue))
    (bind _returnvalue_4 (`KismetMathLibrary.VSizeSquared` _returnvalue_3))
    (if (and (and (>= _angle _negative) (<= _angle _positive)) (and (< _returnvalue_4 (`local.shortest_distance`)) (>= (`KismetMathLibrary.Dot_VectorVector` (`KismetMathLibrary.Normal` _returnvalue) (`KismetMathLibrary.Normal` _returnvalue_3)) 0.0)))
      (set `local.closest_enemy` _array_element)
      (set `local.shortest_distance` _returnvalue_4)))
  (return (`local.closest_enemy`)))

(fn `UserConstructionScript`)