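; Base turret Blueprint that defines the shared functions for turret types: aiming at points, shooting, rotation range and angle queries, and fire-rate scaling.
; Aiming, shooting and setter functions are empty stubs and the rotation queries return zero, leaving turret behavior unimplemented here.
; The only working logic plays one of three laser cues at random as a non-spatialized 2D sound.
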(fn `compute_target_rotation`
  (params (point :type "Vector Structure"))
  (returns (angle :type "Float (double-precision)"))
  (return 0.0))

(fn `get_current_turn_angle`
  (returns (angle :type "Float (double-precision)"))
  (return 0.0))

(fn `get_rotation_range`
  (returns (negative :type "Float (double-precision)") (positive :type "Float (double-precision)"))
  (return 0.0 0.0))

(fn `play_laser_sounds`
  (switch `int` (`KismetMathLibrary.RandomInteger` 3)
    (:`0`
      (`GameplayStatics.PlaySound2D` "/Game/sounds/laserC_Cue.laserC_Cue" 1.0 1.0 0.0 null null))
    (:`1`
      (`GameplayStatics.PlaySound2D` "/Game/sounds/laserC1_Cue.laserC1_Cue" 1.0 1.0 0.0 null null))
    (:`2`
      (`GameplayStatics.PlaySound2D` "/Game/sounds/laserC2_Cue.laserC2_Cue" 1.0 1.0 0.0 null null))))

(fn `rotate_towards_points`
  (params (point :type "Vector Structure") (factor :type "Float (double-precision)")))

(fn `set_firerate_multiplier`
  (params (multiplier :type "Float (double-precision)")))

(fn `set_relative_rotation`
  (params (angle :type "Float (double-precision)")))

(fn `try_shoot`)

(fn `UserConstructionScript`)