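; Triple-barrel laser turret that swivels around its X axis toward a point, within a clamped roll range.
; TryShoot, gated by a cooldown that a fire-rate multiplier adjusts, launches a random-hued Laser_projectile from each spawner at ProjectileSpeed.
; Each shot squashes the barrel cylinders, and Tick advances the shot timer and eases their length back as recoil recovery.
; ComputeRotation finds a target's relative roll by temporarily rotating the sphere, then restoring it.
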(event `self.ReceiveBeginPlay`
  (set `self.shot_cooldown` (`self.default_shot_cooldown`)))

(event `self.ReceiveTick`
  (params (DeltaSeconds :type "Float (single-precision)"))
  (`self.update_timers` DeltaSeconds)
  (`self.restore_scale`))

(event `self.try_shoot`
  ;[1 1 1] shoot
  (if (`self.may_shoot`)
    (set `self.shot_timer` 0.0)
    (`self.spawn_projectile` (`self.projectile_spawner0`) (`self.cylinder0`))
    (`SceneComponent.SetRelativeScale3D` (`self.cylinder0`) (1.0 1.0 0.5))
    (`self.spawn_projectile` (`self.projectile_spawner1`) (`self.cylinder1`))
    (`SceneComponent.SetRelativeScale3D` (`self.cylinder1`) (1.0 1.0 0.5))
    (`self.spawn_projectile` (`self.projectile_spawner2`) (`self.cylinder2`))
    (`SceneComponent.SetRelativeScale3D` (`self.cylinder2`) (1.0 1.0 0.5))
    (`self.play_laser_sounds`)
    (`self.play_laser_sounds`)
    (`self.play_laser_sounds`)))

(event `self.rotate_towards_points`
  (params (point :type "Vector Structure") (factor :type "Float (single-precision)"))
  ;[1 1 1] rotate
  (`SceneComponent.K2_SetWorldRotation` (`self.Sphere`) (`KismetMathLibrary.RotatorFromAxisAndAngle` (1.0 0.0 0.0) (* (`KismetMathLibrary.DegAtan2` (* (.y (- point (`SceneComponent.K2_GetComponentLocation` (`self.DefaultSceneRoot`)))) -1.0) (.z (- point (`SceneComponent.K2_GetComponentLocation` (`self.DefaultSceneRoot`))))) factor)) false false)
  (`SceneComponent.K2_SetRelativeRotation` (`self.Sphere`) (`KismetMathLibrary.MakeRotator` (`KismetMathLibrary.ClampAngle` (.roll (`SceneComponent.RelativeRotation` (`self.Sphere`))) -70.0 70.0)) false false))

(event `self.set_relative_rotation`
  (params (angle :type "Float (single-precision)"))
  (`SceneComponent.K2_SetRelativeRotation` (`self.Sphere`) (`KismetMathLibrary.MakeRotator` angle) false false))

(event `self.set_firerate_multiplier`
  (params (multiplier :type "Float (single-precision)"))
  (set `self.shot_cooldown` (- (`self.default_shot_cooldown`) (* multiplier 0.03))))

(fn `compute_rotation`
  (params (point :type "Vector Structure"))
  (returns (angle :type "Float (double-precision)"))
  (locals (rotation :type "Rotator Structure") (computed_rotation :type "Rotator Structure"))
  (set `local.rotation` (`SceneComponent.K2_GetComponentRotation` (`self.Sphere`)))
  (`SceneComponent.K2_SetWorldRotation` (`self.Sphere`) (`KismetMathLibrary.RotatorFromAxisAndAngle` (1.0 0.0 0.0) (`KismetMathLibrary.DegAtan2` (* (.y (- point (`SceneComponent.K2_GetComponentLocation` (`self.DefaultSceneRoot`)))) -1.0) (.z (- point (`SceneComponent.K2_GetComponentLocation` (`self.DefaultSceneRoot`)))))) false false)
  (bind _output_get (set `local.computed_rotation` (`SceneComponent.RelativeRotation` (`self.Sphere`))))
  (`SceneComponent.K2_SetWorldRotation` (`self.Sphere`) (`local.rotation`) false false)
  (return (.roll _output_get)))

(fn `compute_target_rotation`
  (params (point :type "Vector Structure"))
  (returns (angle :type "Float (double-precision)"))
  (bind _angle (`self.compute_rotation` point))
  (return _angle))

(fn `get_current_turn_angle`
  (returns (angle :type "Float (double-precision)"))
  (return (.roll (`SceneComponent.RelativeRotation` (`self.Sphere`)))))

(fn `get_rotation_range`
  (returns (negative :type "Float (double-precision)") (positive :type "Float (double-precision)"))
  (return -70.0 70.0))

(fn `restore_scale`
  (bind _returnvalue (`KismetMathLibrary.MakeVector` 1.0 1.0 (`|EaseFunction` "CircularOut" (`KismetMathLibrary.FClamp` (/ (`self.shot_timer`) (`self.shot_cooldown`))) 0.5 0.75)))
  (`SceneComponent.SetRelativeScale3D` (`self.cylinder0`) _returnvalue)
  (`SceneComponent.SetRelativeScale3D` (`self.cylinder1`) _returnvalue)
  (`SceneComponent.SetRelativeScale3D` (`self.cylinder2`) _returnvalue))

(fn `set_random_color`
  (params (object :type "PrimitiveComponent Object Reference"))
  (locals (projectile_color :type "LinearColor Structure"))
  (bind _returnvalue (`PrimitiveComponent.CreateDynamicMaterialInstance` object 0 "/Game/geometry/laser_mat.laser_mat" "None"))
  (bind _returnvalue_2 (`MaterialInstanceDynamic.K2_GetVectorParameterValue` _returnvalue "color"))
  (bind _output_get (set `local.projectile_color` _returnvalue_2))
  (`KismetMathLibrary.LinearColor_SetRandomHue` _output_get)
  (`MaterialInstanceDynamic.SetVectorParameterValue` _returnvalue "color" (`local.projectile_color`)))

(fn `spawn_projectile`
  (params (spawner :type "SceneComponent Object Reference") (turret :type "SceneComponent Object Reference"))
  (returns (projectile :type "/Game/blueprints/laser_projectile Object Reference"))
  (bind _direction (`self.compute_shot_direction` spawner turret))
  (bind _returnvalue (`|SpawnActorFromClass` "/Game/blueprints/laser_projectile.laser_projectile_C" (`KismetMathLibrary.MakeTransform` (`SceneComponent.K2_GetComponentLocation` spawner) (struct) (0.2 0.2 0.2)) "Undefined" "OverrideRootScale" null null))
  (bind _laser_beam (`/Game/blueprints/laser_projectile.laser_beam` _returnvalue))
  (`self.set_random_color` _laser_beam)
  (`PrimitiveComponent.SetAllPhysicsLinearVelocity` _laser_beam (* _direction (`self.projectile_speed`)) false)
  (`SceneComponent.K2_SetWorldRotation` _laser_beam (`KismetMathLibrary.RotatorFromAxisAndAngle` (1.0 0.0 0.0) (`KismetMathLibrary.DegAtan2` (* (.y _direction) -1.0) (.z _direction))) false false)
  (return _returnvalue))

(fn `update_timers`
  (params (delta_time :type "Float (double-precision)"))
  (set `self.shot_timer` (+ delta_time (`self.shot_timer`))))

(fn `UserConstructionScript`
  (`parent.UserConstructionScript`))